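; Main player character Blueprint that handles input for a skill panel and a second UI widget.
; BeginPlay creates and stores the skill panel, which K toggles through a FlipFlop, refreshing its levels each time it opens.
; Holding M shows a widget created anew on each press and removed on release.
; Both switch the mouse cursor and input mode between game-and-UI and game-only.
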(event EventBeginPlay
  (bind _returnvalue (UserInterface|CreateWidget "/Game/HUD/SkillPanel.SkillPanel_C"))
  (Variables|Default|SetSkillPanel _returnvalue))

(event Collision|EventActorBeginOverlap
  (params (OtherActor :type Actor%20Object%20Reference)))

(event EventTick
  (params (DeltaSeconds :type Float%20%28single-precision%29)))

(event Input|KeyboardEvents|M
  (params (Key :type Key%20Structure :default "None"))
  (bind _returnvalue (Game|GetPlayerController 0))
  (:Pressed
    (bind _returnvalue_2 (UserInterface|CreateWidget "/Game/UMGMiniMap/Blueprints/UI.UI_C" _returnvalue))
    (UserInterface|Viewport|AddtoViewport _returnvalue_2 0)
    (Variables|/Script/Engine.PlayerController|SetbShowMouseCursor _returnvalue true)
    (Input|SetInputModeGameandUI 0 0 "DoNotLock" true))
  (:Released
    (Widget|RemovefromParent _returnvalue_2)
    (Input|SetInputModeGameOnly _returnvalue)
    (Variables|/Script/Engine.PlayerController|SetbShowMouseCursor _returnvalue false)))

(event Input|KeyboardEvents|K
  (params (Key :type Key%20Structure :default "None"))
  (bind _returnvalue (Game|GetPlayerController 0))
  (bind _skillpanel (Variables|Default|GetSkillPanel))
  (:Pressed
    (Utilities|FlowControl|FlipFlop
      (:A
        (UserInterface|Viewport|AddtoViewport _skillpanel 0)
        (Default|UpdateLevels _skillpanel)
        (Variables|/Script/Engine.PlayerController|SetbShowMouseCursor _returnvalue true)
        (Input|SetInputModeGameandUI _returnvalue _skillpanel "DoNotLock" false))
      (:B
        (Widget|RemovefromParent (Variables|Default|GetSkillPanel))
        (Input|SetInputModeGameOnly _returnvalue)
        (Variables|/Script/Engine.PlayerController|SetbShowMouseCursor _returnvalue false)))))

(fn ConstructionScript)